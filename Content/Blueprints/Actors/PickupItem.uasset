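; PickupItem is a world pickup actor whose look comes from an item data table row and which the player collects by overlap.
; On BeginPlay it looks up the ItemData row and sets the mesh, scale and spawn offset, then writes each of the mesh's materials to slot 0.
; When a Player_BP overlaps the Box, it passes the item data, name, amount and itself to that player's ClientPickup.
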(event OnComponentBeginOverlap(Box)
  (params (OverlappedComponent :type Primitive%20Component%20Object%20Reference) (OtherActor :type Actor%20Object%20Reference) (OtherComp :type Primitive%20Component%20Object%20Reference) (OtherBodyIndex :type Integer) (bFromSweep :type Boolean) (SweepResult :type Hit%20Result%20Structure%20%28by%20ref%29))
  (bind _asplayer_bp (Utilities|Casting|CastToPlayer_BP OtherActor))
  (Default|ClientPickup _asplayer_bp (Variables|Item|GetAmount) (Variables|Item|GetItemData) (Variables|Item|GetItem%20Name) self))

(event EventBeginPlay
  (bind _itemdata (Variables|Item|GetItemData))
  (bind _staticmesh (Variables|Default|GetStaticMesh))
  (bind _returnvalue (Class|DataTableFunctionLibrary|DoesDataTableRowExist (.datatable _itemdata) (.rowname _itemdata)))
  (if _returnvalue
    (bind _returnvalue_2 (Utilities|GetDataTableRow (.datatable _itemdata) (.rowname _itemdata))
      (:then
        (Components|StaticMesh|SetStaticMesh _staticmesh (.StaticMesh (Utilities|Struct|BreakInventoryStructure _returnvalue_2)))
        (Transformation|SetWorldScale3D _staticmesh (* "0.500000,0.500000,0.500000" (.Scale (Utilities|Struct|BreakInventoryStructure _returnvalue_2))))
        (Transformation|SetWorldLocation (Variables|Default|GetStaticMesh) (+ (Transformation|GetWorldLocation (Variables|Default|GetStaticMesh)) (.SpawnOffset (Utilities|Struct|BreakInventoryStructure _returnvalue_2))) false false)
        (for _array_element (Variables|/Script/Engine.StaticMesh|GetStaticMaterials (.StaticMesh (Utilities|Struct|BreakInventoryStructure _returnvalue_2)))
          (Rendering|Material|SetMaterial _staticmesh 0 (.MaterialInterface (Utilities|Struct|BreakStaticMaterial _array_element))))))))

(fn ConstructionScript)