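; FireBall_BP is a short-lived fireball actor that damages any Player_BP overlapping its Sphere and destroys itself after 1.2 seconds.
; On a player hit it applies fixed damage, spawns an enlarged explosion emitter, disables Sphere collision and hides its particle system.
; A brief delay then removes the explosion and the actor, though the BeginPlay lifetime timer still runs and can destroy the actor first.
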(event OnComponentBeginOverlap(Sphere)
  (params (OverlappedComponent :type Primitive%20Component%20Object%20Reference) (OtherActor :type Actor%20Object%20Reference) (OtherComp :type Primitive%20Component%20Object%20Reference) (OtherBodyIndex :type Integer) (bFromSweep :type Boolean) (SweepResult :type Hit%20Result%20Structure%20%28by%20ref%29))
  (bind _asplayer_bp (Utilities|Casting|CastToPlayer_BP OtherActor))
  (Game|Damage|ApplyDamage _asplayer_bp 4e+01 0 self)
  (bind _returnvalue (Effects|SpawnEmitteratLocation "/Game/Assets/StarterContent/Particles/P_Explosion.P_Explosion" (Transformation|GetActorLocation) "0, 0, 0" "2.000000,2.000000,2.000000"))
  (Collision|SetCollisionEnabled (Variables|Default|GetSphere) "NoCollision")
  (Rendering|SetVisibility (Variables|Default|GetParticleSystem) false false)
  (Utilities|FlowControl|Delay 0.5)
  (Components|DestroyComponent _returnvalue)
  (Actor|DestroyActor))

(event Collision|EventActorBeginOverlap
  (params (OtherActor :type Actor%20Object%20Reference)))

(event EventTick
  (params (DeltaSeconds :type Float%20%28single-precision%29)))

(event EventBeginPlay
  (Utilities|FlowControl|Delay 1.2)
  (Actor|DestroyActor))

(fn ConstructionScript)