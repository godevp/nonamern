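; AI controller for monsters that runs BT_Monster on BeginPlay and reacts to perception of the player.
; Perception updates store the actor and stimulus, check the sense class name, then call SightFunc.
; For a Player_BP actor, SightFunc records CanSee, writes the actor to the blackboard and sets the controlled Zombie_BP's walk speed to a fixed value, even when sight is lost.
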(event OnTargetPerceptionUpdated(AIPerception)
  (params (Actor :type Actor%20Object%20Reference) (Stimulus :type AI%20Stimulus%20Structure))
  (Variables|Default|SetActor Actor)
  (bind _output_get (Variables|Default|SetStimulus Stimulus))
  (bind _returnvalue (Class|AIPerceptionSystem|GetSenseClassforStimulus _output_get))
  (switch string (Utilities|GetClassDisplayName _returnvalue)
    (:AISense_Sight
      (CallFunction|SightFunc))))

(event EventBeginPlay
  (AI|RunBehaviorTree "/Game/Blueprints/Monsters/BT_Monster.BT_Monster"))

(event EventTick
  (params (DeltaSeconds :type Float%20%28single-precision%29)))

(fn ConstructionScript)

(fn SightFunc
  (bind _actor (Variables|Default|GetActor)
    (:then
      (if (== (Utilities|GetClass _actor) "/Game/Blueprints/Player/Player_BP.Player_BP_C")
        (Variables|Default|SetCanSee (.bsuccessfullysensed (Variables|Default|GetStimulus)))
        (AI|Components|Blackboard|SetValueasObject (AI|GetBlackboard 0) (Variables|Default|GetBBboolName) (Variables|Default|GetActor))
        (bind _charactermovement (Variables|/Script/Engine.Character|GetCharacterMovement (.AsZombie%20BP (Utilities|Casting|CastToZombie_BP (Pawn|GetControlledPawn))))
          (:then
            (Variables|/Script/Engine.CharacterMovementComponent|SetMaxWalkSpeed _charactermovement 6e+02))
          (:else))))
    (:else)))