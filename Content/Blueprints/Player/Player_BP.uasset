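; Multiplayer player character with movement, stamina-draining sprint, fireball attack, health potions, item pickup and respawn at a random navigable point.
; Input runs client events that call server events for sprint speed, rotation, delayed camera-aimed fireball spawning, damage and pickup cleanup.
; BeginPlay creates the HUD and in-game menu, has the authority randomize a dark body color applied via OnRep, and loops player-ID name tag updates.
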(fn ConstructionScript)

(fn OnRepBodyColor
  (bind _returnvalue (Rendering|Material|CreateDynamicMaterialInstance (Variables|Character|GetMesh) 0 "/Game/Assets/Characters/NinjaMage/Ch24_Body.Ch24_Body" "None" :!class /Script/Engine.PrimitiveComponent))
  (Rendering|Material|SetVectorParameterValue _returnvalue "BodyColor" (Variables|Default|GetBodyColor) :!class /Script/Engine.MaterialInstanceDynamic))

(event Custom|Use%20Item
  (params (Inventory :type Inventory%20Component%20Object%20Reference))
  (bind _currentitem (Variables|Default|GetCurrentItem))
  (bind (_value _returnvalue) (Utilities|Map|Find (Variables|/Game/Blueprints/Components/Inventory/InventoryComponent.InventoryComponent_C|GetInventory Inventory) _currentitem))
  (if _returnvalue
    (if (>= _value 0)
      (bind _result (Math|Integer|DecrementInt _value)
        (:%20%20
          (Variables|Stats|SetHealth (+ (Variables|Stats|GetHealth) 2e+02))
          (Development|PrintString (Utilities|String|Append (Utilities|String|ToString(Integer) _value) " : Health Potions"))
          (Utilities|Map|Add (Variables|/Game/Blueprints/Components/Inventory/InventoryComponent.InventoryComponent_C|GetInventory Inventory) (Variables|Default|GetCurrentItem) _result))))))

(event Custom|ClientPickup
  (params (Amount :type Integer) (Item%20Data :type Data%20Table%20Row%20Handle%20Structure) (Item%20Name :type Name) (Item%20Ref :type Pickup%20Item%20Object%20Reference))
  (Default|AddtoInventory (Variables|Default|GetInventoryComponent) Item%20Name Amount)
  (CallFunction|ServerCleanupActor Item%20Ref)
  (Utilities|IsValid Item%20Ref
    (:Is%20Valid
      (Actor|DestroyActor Item%20Ref))))

(event Custom|Server_CleanupActor
  (params (Actor :type Actor%20Object%20Reference))
  (Actor|DestroyActor Actor))

(event Input|ActionEvents|InputActionUseItem
  (params (Key :type Key%20Structure :default "None"))
  (:Pressed
    (CallFunction|UseItem (Variables|Default|GetInventoryComponent))))

(event Custom|Client_CloseInGameMenu
  (bind _returnvalue (Game|GetPlayerController 0))
  (bind _gamemenu (Variables|Default|GetGameMenu)
    (:then
      (Widget|SetVisibility _gamemenu "Collapsed")
      (Variables|Default|SetOpenInGameMenu false)
      (Variables|/Script/Engine.PlayerController|SetbShowMouseCursor _returnvalue false)
      (Input|SetInputModeGameOnly _returnvalue))
    (:else)))

(event Custom|Client_OpenInGameMenu
  (bind _returnvalue (Game|GetPlayerController 0))
  (bind _gamemenu (Variables|Default|GetGameMenu)
    (:then
      (Widget|SetVisibility _gamemenu "Visible")
      (Variables|Default|SetOpenInGameMenu true)
      (Variables|/Script/Engine.PlayerController|SetbShowMouseCursor _returnvalue true)
      (Input|SetInputModeGameandUI _returnvalue _gamemenu "DoNotLock" false))
    (:else)))

(event Input|ActionEvents|InputActionInGameMenu
  (params (Key :type Key%20Structure))
  (:Pressed
    (if (Variables|Default|GetOpenInGameMenu)
      (CallFunction|ClientCloseinGameMenu)
      (else
        (CallFunction|ClientOpeninGameMenu)))))

(event Custom|Server_StopSprint
  (Variables|/Script/Engine.CharacterMovementComponent|SetMaxWalkSpeed (Variables|Character|GetCharacterMovement) 4e+02))

(event Custom|Server_Sprint
  (Variables|/Script/Engine.CharacterMovementComponent|SetMaxWalkSpeed (Variables|Character|GetCharacterMovement) 8e+02))

(event Input|ActionEvents|InputActionSprint
  (params (Key :type Key%20Structure :default "None"))
  (bind _charactermovement (Variables|Character|GetCharacterMovement))
  (:Pressed
    (Variables|/Script/Engine.CharacterMovementComponent|SetMaxWalkSpeed _charactermovement 8e+02)
    (Variables|Default|SetisSprinting true)
    (CallFunction|ServerSprint))
  (:Released
    (Variables|/Script/Engine.CharacterMovementComponent|SetMaxWalkSpeed _charactermovement 4e+02)
    (Variables|Default|SetisSprinting false)
    (CallFunction|ServerStopSprint)))

(event Input|ActionEvents|InputActionJump
  (params (Key :type Key%20Structure :default "None"))
  ;[0.552 0.9216 1 0.4078] Movement
  (:Pressed
    (if (and (not (Variables|Default|GetisDead)) (not (Variables|Default|GetOpenInGameMenu)))
      (Character|Jump)))
  (:Released
    (Character|StopJumping)))

(event Input|AxisEvents|InputAxisMoveForward/Backward
  (params (AxisValue :type Float%20%28single-precision%29))
  ;[0.552 0.9216 1 0.4078] Movement
  (if (and (not (Variables|Default|GetisDead)) (not (Variables|Default|GetOpenInGameMenu)))
    (Pawn|Input|AddMovementInput (Math|Vector|GetForwardVector (Math|Rotator|MakeRotator 0.0 0.0 (.yaw (Pawn|GetControlRotation :!class /Script/Engine.Pawn)))) AxisValue false)))

(event Input|AxisEvents|InputAxisTurnRight/LeftMouse
  (params (AxisValue :type Float%20%28single-precision%29))
  ;[0.552 0.9216 1 0.4078] Camera
  (if (not (Variables|Default|GetOpenInGameMenu))
    (Pawn|Input|AddControllerYawInput AxisValue)))

(event Input|AxisEvents|InputAxisLookUp/DownMouse
  (params (AxisValue :type Float%20%28single-precision%29))
  ;[0.552 0.9216 1 0.4078] Camera
  (if (not (Variables|Default|GetOpenInGameMenu))
    (Pawn|Input|AddControllerPitchInput AxisValue)))

(event Input|AxisEvents|InputAxisMoveRight/Left
  (params (AxisValue :type Float%20%28single-precision%29))
  (bind _returnvalue (Pawn|GetControlRotation :!class /Script/Engine.Pawn))
  ;[0.552 0.9216 1 0.4078] Movement
  (if (and (not (Variables|Default|GetisDead)) (not (Variables|Default|GetOpenInGameMenu)))
    (Pawn|Input|AddMovementInput (Math|Vector|GetRightVector (Math|Rotator|MakeRotator (.roll _returnvalue) 0.0 (.yaw _returnvalue))) AxisValue false)))

(event EventBeginPlay
  (bind _returnvalue (Game|GetPlayerController 0))
  ;[0.1892 1 0.0502 0.281] BeginPlay
  (Utilities|FlowControl|Sequence
    (:then_0
      (bind _returnvalue_2 (Game|GetCurrentLevelName true))
      (if (Utilities|Enum|NotEqual(Enum) _returnvalue_2 "MainMenu_map")
        (if (Pawn|IsLocallyControlled)
          (Input|SetInputModeGameOnly _returnvalue)
          (Variables|/Script/Engine.PlayerController|SetbShowMouseCursor _returnvalue false)
          (bind _returnvalue_3 (UserInterface|CreateWidget "/Game/Blueprints/Widgets/UI.UI_C" (Game|GetPlayerController 0)))
          (Variables|Default|SetUI%20widget _returnvalue_3)
          (bind _ui_widget (Variables|Default|GetUI%20widget)
            (:then
              (UserInterface|Viewport|AddtoViewport _ui_widget 0)
              (Variables|/Game/Blueprints/Widgets/UI.UI_C|SetOwner (Variables|Default|GetUI%20widget) self))
            (:else)))))
    (:then_1
      (bind _returnvalue_4 (UserInterface|CreateWidget "/Game/Blueprints/Widgets/InGameMenu_widget.InGameMenu_widget_C"))
      (Variables|Default|SetGameMenu _returnvalue_4)
      (bind _gamemenu (Variables|Default|GetGameMenu)
        (:then
          (UserInterface|Viewport|AddtoViewport _gamemenu 0)
          (Widget|SetVisibility _gamemenu "Collapsed")
          (Variables|/Game/Blueprints/Widgets/InGameMenu_widget.InGameMenu_widget_C|SetOwner _gamemenu self))
        (:else)))
    (:then_2
      ;;[0.005182 0 0] third frame(without it we will get error)
      (Utilities|FlowControl|Delay 2.0)
      (CallFunction|ClientSetPlayerName :!label _label)
      (Utilities|FlowControl|Delay 5.0)
      (goto _label))
    (:then_3
      ;;[0.005182 0 0] Set different color for each player
      (Networking|SwitchHasAuthority
        (:Authority
          (Variables|Default|SetBodyColor (Utilities|Struct|MakeLinearColor (Math|Random|RandomFloatinRange 0.0 0.07) (Math|Random|RandomFloatinRange 0.0 0.07) (Math|Random|RandomFloatinRange 0.0 0.07) 0.0)))))))

(event EventTick
  (params (DeltaSeconds :type Float%20%28single-precision%29))
  ;[1 0 0.01969 0.187] Update
  (if (Variables|Default|GetisSprinting)
    (Variables|Default|SetStamina (Math|Float|Clamp(Float) (- (Variables|Default|GetStamina) (* 1e+01 (Utilities|Time|GetWorldDeltaSeconds))) 0.0 (Variables|Default|GetMaxStamina)))))

(event Custom|Server_isAttacking
  (Variables|Default|SetisAttacking true)
  (Utilities|FlowControl|Delay 1.51)
  (Variables|Default|SetisAttacking false))

(event Custom|Server_ApplyDamage
  (params (Damage :type Float%20%28double-precision%29) (DamagedActor :type Actor%20Object%20Reference) (DamageCauser :type Actor%20Object%20Reference))
  ;[0 0.005182 0] Server Damage Applier (Can use in other blueprints)
  (Game|Damage|ApplyDamage DamagedActor Damage 0 DamageCauser))

(event Custom|Server_CreateFireBall
  (params (Spawn%20Transform%20Location :type Vector) (Spawn%20Transform%20Rotation :type Rotator))
  ;[1 0.1605 0.09082 0.156] FireBallCreation
  ;;[0 0.005182 0] Third (The server action) - the action itself for the whole server so everybody will see it
  (bind _returnvalue (Game|SpawnActorfromClass "/Game/Blueprints/Player/FireBall_BP.FireBall_BP_C" (Math|Transform|MakeTransform Spawn%20Transform%20Location Spawn%20Transform%20Rotation "1.000000,1.000000,1.000000") "Undefined" 0 0))
  (Variables|/Game/Blueprints/Player/FireBall_BP.FireBall_BP_C|SetOwneeer _returnvalue self))

(event Custom|Server_SetActorRotation
  (params (New%20rotation :type Rotator))
  ;[1 0.1605 0.09082 0.156] FireBallCreation
  ;;[0 0.005182 0] Server SetActorRotation
  (Transformation|SetActorRotation New%20rotation))

(event Custom|Client_Fire
  (params (Camera :type Camera%20Component%20Object%20Reference))
  (bind _returnvalue (Transformation|GetActorLocation))
  ;[1 0.1605 0.09082 0.156] FireBallCreation
  ;;[0 0.005182 0] Second (The client action) - Pass the calculations made in client to the server action
  (if (not (Variables|Default|GetisAttacking))
    (CallFunction|ServerIsAttacking)
    (Utilities|FlowControl|Delay 0.8)
    (bind _output_get (Variables|Default|SetStartCameraShootLoc (Math|Vector|GetForwardVector Camera)))
    (bind _output_get_2 (Variables|Default|SetStartCameraRot (Transformation|GetWorldRotation Camera)))
    (|SetActorrotationinclientandserver_2 Camera)
    (CallFunction|ServerCreateFireBall (+ (* _output_get "100.000000,100.000000,100.000000") (Math|Vector|MakeVector (.x _returnvalue) (.y _returnvalue) (+ (.z _returnvalue) 5e+01))) (Math|Rotator|MakeRotator (.roll _output_get_2) (+ (.pitch _output_get_2) 3.0) (.yaw _output_get_2)))))

(event Game|Damage|EventAnyDamage
  (params (Damage :type Float%20%28single-precision%29) (DamageType :type Damage%20Type%20Object%20Reference) (InstigatedBy :type Controller%20Object%20Reference) (DamageCauser :type Actor%20Object%20Reference))
  ;[0 0.005182 0] Any damage taken
  (if (> (Variables|Stats|GetHealth) 0.0)
    (Variables|Stats|SetHealth (- (Variables|Stats|GetHealth) Damage))
    (if (<= (Variables|Stats|GetHealth) 0.0)
      (Variables|Stats|SetHealth 0.0)
      (Variables|Default|SetisDead true)
      (CallFunction|ClientRespawn))))

(event Input|ActionEvents|InputActionFire
  (params (Key :type Key%20Structure :default "None"))
  ;[1 0.1605 0.09082 0.156] FireBallCreation
  ;;[0 0.005182 0] First - trigger the client action
  (:Pressed
    (if (Math|Boolean|ANDBoolean (not (Variables|Default|GetisDead)) (not (Variables|Default|GetOpenInGameMenu)) (not (AI|Components|NavMovement|IsFalling (Variables|Character|GetCharacterMovement))))
      (CallFunction|ClientFire (Variables|Default|GetCamera)))))

(event Input|KeyboardEvents|X
  (params (Key :type Key%20Structure :default "None")))

(event Custom|Client_Respawn
  ;[0 0.005182 0] Client respawn
  (Variables|Stats|SetHealth 1e+03)
  (Variables|Default|SetisDead false)
  (bind _randomlocation (Class|NavigationSystemV1|GetRandomLocationinNavigableRadius (Math|Vector|MakeVector 0.0 0.0 0.0) 1e+04 0 0))
  (Transformation|SetActorLocation _randomlocation false true))

(event Custom|Client_SetPlayerName
  ;[0 0.005182 0] Client set player names
  (bind _outactors (Actor|GetAllActorsOfClass "Player_BP_C"))
  (for _array_element _outactors
    (bind _playerstate (Variables|/Script/Engine.Pawn|GetPlayerState _array_element)
      (:then
        (Rendering|Components|TextRender|SetText (Variables|Player_BP_C|GetPlayerName _array_element) (Utilities|Text|ToText(String) (Utilities|String|Append "PlayerID: " (Utilities|String|ToString(Integer) (Variables|/Script/Engine.PlayerState|GetPlayerId _playerstate))))))
      (:else))))